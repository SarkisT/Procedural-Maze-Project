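; MazeBP is the maze game's rule Blueprint, ending play when the MazeCharacter reaches three points or a countdown expires.
; Tick looks up the character each frame and, on a win, pauses, prints a message, shows the cursor and switches to UI-only input.
; A one-second Delay inside Tick decrements Timer; at zero it pauses and re-enters the check, printing the loss message with the same cursor handoff.
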(event EventBeginPlay)

(event Collision|EventActorBeginOverlap
  (params (OtherActor :type Actor%20Object%20Reference)))

(event EventTick
  (params (DeltaSeconds :type Float%20%28single-precision%29))
  (bind _returnvalue (Game|GetPlayerController 0))
  (Utilities|FlowControl|Sequence
    (:then_0
      (bind _returnvalue_2 (Actor|GetActorOfClass "/Script/Maze.MazeCharacter" :!label _label))
      (if (== (Variables|/Script/Maze.MazeCharacter|Getpoints _returnvalue_2) 3)
        (Game|SetGamePaused true)
        (Development|PrintString "Hello")
        (Variables|/Script/Engine.PlayerController|SetbShowMouseCursor _returnvalue true :!label _label_2)
        (Input|SetInputModeUIOnly _returnvalue 0 "DoNotLock")
        (elif (Variables|Default|GetTimer%20Condition)
          (Development|PrintString "Bye")
          (goto _label_2))))
    (:then_1
      (Utilities|FlowControl|Delay 1.0)
      (bind _output_get (Variables|Default|SetTimer (- (Variables|Default|GetTimer) 1)))
      (bind _output_get_2 (Variables|Default|SetTimer%20Condition (<= _output_get 0)))
      (if _output_get_2
        (Game|SetGamePaused true)
        (goto _label)))))

(fn ConstructionScript)